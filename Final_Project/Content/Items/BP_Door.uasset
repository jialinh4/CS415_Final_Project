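; BP_Door is an exit door that ends the game once two player characters meet the win conditions.
; When its mesh is hit by a ThirdPersonCharacter, it finds all actors of that class and reads the first two.
; If their combined NumKey equals two and both have PlayerEnd set, it shows the GameEnd_WBP widget, waits briefly, then opens NewMap.
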(event `self.SM_MatPreviewMesh_02.OnComponentHit`
  (params (HitComponent :type "PrimitiveComponent Object Reference") (OtherActor :type "Actor Object Reference") (OtherComp :type "PrimitiveComponent Object Reference") (NormalImpulse :type "Vector Structure") (Hit :type "HitResult Structure (by ref)"))
  (bind _asthird_person_character (castclass `/Game/ThirdPersonBP/Blueprints/ThirdPersonCharacter` (`GameplayStatics.GetObjectClass` OtherActor)))
  (bind _outactors (`GameplayStatics.GetAllActorsOfClass` _asthird_person_character))
  (bind _output (`|GetArrayItem` _outactors))
  (bind _output_2 (`|GetArrayItem` _outactors 1))
  (if (and (== (+ (`/Game/ThirdPersonBP/Blueprints/ThirdPersonCharacter.numKey` _output) (`/Game/ThirdPersonBP/Blueprints/ThirdPersonCharacter.numKey` _output_2)) 2) (and (`/Game/ThirdPersonBP/Blueprints/ThirdPersonCharacter.PlayerEnd` _output) (`/Game/ThirdPersonBP/Blueprints/ThirdPersonCharacter.PlayerEnd` _output_2)))
    (bind _returnvalue (`|CreateWidget` "/Game/UI/GameEnd_WBP.GameEnd_WBP_C"))
    (`UserWidget.AddToViewport` _returnvalue 0)
    (`KismetSystemLibrary.Delay` 2.0)
    (`GameplayStatics.OpenLevel` "NewMap")))

(fn `UserConstructionScript`)